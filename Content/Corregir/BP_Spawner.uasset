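; BP_Spawner is an actor that repeatedly spawns BP_ObjetoMovil1 actors at its own transform while the game has started.
; Tick reads the GameStart flag on the player's BP_FirstPersonCharacter and, when it is set, calls the GameStart event, which checks the flag again.
; That event accumulates delta time, then spawns and resets the timer each time it reaches SpawnInterval.
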(event Custom|GameStart
  (bind _asbp_first_person_character (Utilities|Casting|CastToBP_FirstPersonCharacter (Game|GetPlayerCharacter 0)))
  (if (Variables|/Game/Corregir/BP_FirstPersonCharacter.BP_FirstPersonCharacter_C|GetGameStart _asbp_first_person_character)
    (Variables|Default|SetTimeSinceLastSpawn (+ (Utilities|Time|GetWorldDeltaSeconds) (Variables|Default|GetTimeSinceLastSpawn)))
    (if (>= (Variables|Default|GetTimeSinceLastSpawn) (Variables|Default|GetSpawnInterval))
      (Game|SpawnActorfromClass "/Game/Corregir/BP_ObjetoMovil1.BP_ObjetoMovil1_C" (Transformation|GetActorTransform) "Undefined" "MultiplyWithRoot" 0 0)
      (Variables|Default|SetTimeSinceLastSpawn 0.0))))

(event EventBeginPlay)

(event Collision|EventActorBeginOverlap
  (params (OtherActor :type Actor%20Object%20Reference)))

(event EventTick
  (params (DeltaSeconds :type Float%20%28single-precision%29))
  (bind _asbp_first_person_character (Utilities|Casting|CastToBP_FirstPersonCharacter (Game|GetPlayerCharacter 0)))
  (if (Variables|/Game/Corregir/BP_FirstPersonCharacter.BP_FirstPersonCharacter_C|GetGameStart _asbp_first_person_character)
    (CallFunction|GameStart)))

(fn ConstructionScript)