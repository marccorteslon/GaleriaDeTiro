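; BP_ObjetoMovil2 is a moving target that awards points when shot and penalizes the player when it expires.
; Tick moves it along local X at a frame-rate-dependent speed, while a Delay throttles the Duracion countdown to roughly once per second.
; A projectile Hit adds to the player character's Puntuacion; timeout calls RestarPuntos to subtract, both destroying the actor and printing the score.
; MostrarPuntos prints a hardcoded message and is uncalled here.
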(event Custom|RestarPuntos
  (bind _asbp_first_person_character (Utilities|Casting|CastToBP_FirstPersonCharacter (Game|GetPlayerCharacter 0)))
  (bind _output_get (Variables|Default|SetAs%20BP%20First%20Person%20Character _asbp_first_person_character))
  (Variables|/Game/Corregir/BP_FirstPersonCharacter.BP_FirstPersonCharacter_C|SetPuntuacion _output_get (- (Variables|/Game/Corregir/BP_FirstPersonCharacter.BP_FirstPersonCharacter_C|GetPuntuacion _output_get) (Variables|Default|GetPuntuacionRestada)))
  (Actor|DestroyActor)
  (Development|PrintText (Utilities|Text|FormatText "Has perdido {0} puntos, llevas {1}" (Variables|Default|GetPuntuacionRestada) (Variables|/Game/Corregir/BP_FirstPersonCharacter.BP_FirstPersonCharacter_C|GetPuntuacion _asbp_first_person_character)) true true "(R=0.807843,G=0.047059,B=0.000000,A=1.000000)"))

(event Custom|MostrarPuntos
  (bind _asbp_first_person_character (Utilities|Casting|CastToBP_FirstPersonCharacter (Game|GetPlayerCharacter 0)))
  (Development|PrintText "Has ganado 10 puntos, llevas ")
  (Development|PrintText (Utilities|Text|ToText(Integer) (Variables|/Game/Corregir/BP_FirstPersonCharacter.BP_FirstPersonCharacter_C|GetPuntuacion _asbp_first_person_character))))

(event Collision|EventActorBeginOverlap
  (params (OtherActor :type Actor%20Object%20Reference)))

(event EventTick
  (params (DeltaSeconds :type Float%20%28single-precision%29))
  (Transformation|AddActorLocalOffset "5.000000,0.000000,0.000000" false false)
  (Utilities|FlowControl|Delay 1.0)
  (Variables|Default|SetDuracion (- (Variables|Default|GetDuracion) 1))
  (if (<= (Variables|Default|GetDuracion) 0)
    (CallFunction|RestarPuntos)))

(event Collision|EventHit
  (params (MyComp :type Primitive%20Component%20Object%20Reference) (Other :type Actor%20Object%20Reference) (OtherComp :type Primitive%20Component%20Object%20Reference) (bSelfMoved :type Boolean) (HitLocation :type Vector :default "0, 0, 0") (HitNormal :type Vector :default "0, 0, 0") (NormalImpulse :type Vector :default "0, 0, 0") (Hit :type Hit%20Result%20Structure%20%28by%20ref%29))
  (Utilities|Casting|CastToBP_FirstPersonProjectile Other)
  (bind _asbp_first_person_character (Utilities|Casting|CastToBP_FirstPersonCharacter (Game|GetPlayerCharacter 0)))
  (bind _output_get (Variables|Default|SetAs%20BP%20First%20Person%20Character _asbp_first_person_character))
  (Variables|/Game/Corregir/BP_FirstPersonCharacter.BP_FirstPersonCharacter_C|SetPuntuacion _output_get (+ (Variables|/Game/Corregir/BP_FirstPersonCharacter.BP_FirstPersonCharacter_C|GetPuntuacion _output_get) (Variables|Default|GetPuntuacionAñadida)))
  (Actor|DestroyActor)
  (Development|PrintText (Utilities|Text|FormatText "Has ganado {0} puntos, llevas {1}" (Variables|Default|GetPuntuacionAñadida) (Variables|/Game/Corregir/BP_FirstPersonCharacter.BP_FirstPersonCharacter_C|GetPuntuacion _asbp_first_person_character))))

(fn ConstructionScript)