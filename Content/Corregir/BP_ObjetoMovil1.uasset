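; Moving shooting target that awards points to the player's score when shot and deducts points if it times out.
; Tick slides it along local X by a fixed per-frame offset, using a Delay to count Duracion down about once per second until RestarPuntos runs.
; A BP_FirstPersonProjectile hit adds PuntuacionAñadida to the character's Puntuacion, while RestarPuntos subtracts PuntuacionRestada.
; Both outcomes destroy the actor and print the change and total.
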(event Collision|EventActorBeginOverlap
  (params (OtherActor :type Actor%20Object%20Reference)))

(event EventTick
  (params (DeltaSeconds :type Float%20%28single-precision%29))
  ;[1 1 1] Se mueve hacia X, y si al pasar un tiempo no se destruye, llama a la función RestarPuntos
  (Transformation|AddActorLocalOffset "5.000000,0.000000,0.000000" false false)
  (Utilities|FlowControl|Delay 1.0)
  (Variables|Default|SetDuracion (- (Variables|Default|GetDuracion) 1))
  (if (<= (Variables|Default|GetDuracion) 0)
    (CallFunction|RestarPuntos)))

(event Collision|EventHit
  (params (MyComp :type Primitive%20Component%20Object%20Reference) (Other :type Actor%20Object%20Reference) (OtherComp :type Primitive%20Component%20Object%20Reference) (bSelfMoved :type Boolean) (HitLocation :type Vector :default "0, 0, 0") (HitNormal :type Vector :default "0, 0, 0") (NormalImpulse :type Vector :default "0, 0, 0") (Hit :type Hit%20Result%20Structure%20%28by%20ref%29))
  ;[1 1 1] Cuando es alcanzado, se destruye, luego te suma puntos y te los muestra + los que llevas
  (Utilities|Casting|CastToBP_FirstPersonProjectile Other)
  (bind _asbp_first_person_character (Utilities|Casting|CastToBP_FirstPersonCharacter (Game|GetPlayerCharacter 0)))
  (bind _output_get (Variables|Default|SetAs%20BP%20First%20Person%20Character _asbp_first_person_character))
  (Variables|/Game/Corregir/BP_FirstPersonCharacter.BP_FirstPersonCharacter_C|SetPuntuacion _output_get (+ (Variables|/Game/Corregir/BP_FirstPersonCharacter.BP_FirstPersonCharacter_C|GetPuntuacion _output_get) (Variables|Default|GetPuntuacionAñadida)))
  (Actor|DestroyActor)
  (Development|PrintText (Utilities|Text|FormatText "Has ganado {0} puntos, llevas {1}" (Variables|Default|GetPuntuacionAñadida) (Variables|/Game/Corregir/BP_FirstPersonCharacter.BP_FirstPersonCharacter_C|GetPuntuacion _asbp_first_person_character))))

(fn ConstructionScript)

(fn RestarPuntos
  ;[1 1 1] Cuando se llama a esta funcion, te resta puntos y te los muestra + los que llevas
  (bind _asbp_first_person_character (Utilities|Casting|CastToBP_FirstPersonCharacter (Game|GetPlayerCharacter 0)))
  (bind _output_get (Variables|Default|SetAs%20BP%20First%20Person%20Character _asbp_first_person_character))
  (Variables|/Game/Corregir/BP_FirstPersonCharacter.BP_FirstPersonCharacter_C|SetPuntuacion _output_get (- (Variables|/Game/Corregir/BP_FirstPersonCharacter.BP_FirstPersonCharacter_C|GetPuntuacion _output_get) (Variables|Default|GetPuntuacionRestada)))
  (Actor|DestroyActor)
  (Development|PrintText (Utilities|Text|FormatText "Has perdido {0} puntos, llevas {1}" (Variables|Default|GetPuntuacionRestada) (Variables|/Game/Corregir/BP_FirstPersonCharacter.BP_FirstPersonCharacter_C|GetPuntuacion _asbp_first_person_character)) true true "(R=0.807843,G=0.047059,B=0.000000,A=1.000000)"))